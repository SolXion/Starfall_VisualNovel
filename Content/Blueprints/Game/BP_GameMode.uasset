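; Game mode Blueprint that applies graphics scalability settings at startup and handles a pause menu event.
; BeginPlay creates a pause menu widget but sets GameUI to None before calling AddToViewport on it.
; PauseGame branches on paused state to clear or push UI_PauseMenu_Root on GameUI's PauseStack, switching input mode.
; Both branches call SetGamePaused(false) and hide the cursor; the menu branch also centers the mouse.
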(event Custom|PauseGame
  (bind _returnvalue (Viewport|GetViewportSize))
  (bind _returnvalue_2 (Game|GetPlayerController 0))
  (bind _gameui (Variables|Default|GetGameUI))
  (bind _pausestack (Variables|/Game/Blueprints/UI/UI_GameUI.UI_GameUI_C|GetPauseStack _gameui))
  (if (Game|IsGamePaused)
    (Game|SetGamePaused false)
    (Class|CommonActivatableWidgetContainerBase|ClearWidgets _pausestack)
    (Input|SetInputModeGameOnly _returnvalue_2 false)
    (Variables|/Script/Engine.PlayerController|SetbShowMouseCursor _returnvalue_2 false)
    (else
      (Game|SetGamePaused false)
      (bind _returnvalue_3 (Class|CommonActivatableWidgetContainerBase|AddWidget _pausestack "/Game/Blueprints/PauseMenu/UI_PauseMenu_Root.UI_PauseMenu_Root_C"))
      (Input|SetInputModeGameandUI _returnvalue_2 _returnvalue_3 "DoNotLock" true false)
      (Variables|/Script/Engine.PlayerController|SetbShowMouseCursor _returnvalue_2 false)
      (Class|PlayerController|SetMouseLocation _returnvalue_2 (Math|Float|Truncate (/ (.x _returnvalue) 2.0)) (Math|Float|Truncate (/ (.y _returnvalue) 2.0))))))

(event EventBeginPlay
  (bind _returnvalue (Settings|GetGameUserSettings))
  (Class|GameUserSettings|SetOverallScalabilityLevel _returnvalue 2)
  (Class|GameUserSettings|ApplySettings _returnvalue true)
  (UserInterface|CreateWidget "/Game/Blueprints/PauseMenu/UI_PauseMenu_Root.UI_PauseMenu_Root_C")
  (bind _output_get (Variables|Default|SetGameUI 0))
  (UserInterface|Viewport|AddtoViewport _output_get 0))

(fn ConstructionScript)