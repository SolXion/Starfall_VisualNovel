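; Game instance for Starfall that owns the persistent settings save and applies saved audio volumes at startup.
; On init it loads the Settings slot, or creates and saves a new BP_SaveSettings if none exists.
; It polls until a game mode is valid, then pushes a sound mix with Master, Music and SFX volume overrides.
; It exposes the settings through a getter and saves them on shutdown.
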(event EventInit
  (bind _returnvalue (SaveGame|DoesSaveGameExist "Settings"))
  (if _returnvalue
    (bind _returnvalue_2 (SaveGame|LoadGamefromSlot "Settings"))
    (bind _asbp_save_settings (Utilities|Casting|CastToBP_SaveSettings _returnvalue_2))
    (Variables|Default|SetSaveSettings _asbp_save_settings)
    (else
      (bind _returnvalue_3 (SaveGame|CreateSaveGameObject "/Game/Blueprints/SoundSettings/BP_SaveSettings.BP_SaveSettings_C"))
      (bind _output_get (Variables|Default|SetSaveSettings _returnvalue_3))
      (SaveGame|SaveGametoSlot _output_get "Settings")))
  (Utilities|IsValid (Game|GetGameMode) :!label _label
    (:Is%20Valid
      (Audio|SetSoundMixClassOverride "/Game/Blueprints/SoundSettings/Sounds/SCM_Main.SCM_Main" "/Game/Blueprints/SoundSettings/Sounds/SC_Master.SC_Master" (Variables|/Game/Blueprints/SoundSettings/BP_SaveSettings.BP_SaveSettings_C|GetMasterVolume (Variables|Default|GetSaveSettings)) 1.0 1.0 true)
      (Audio|SetSoundMixClassOverride "/Game/Blueprints/SoundSettings/Sounds/SCM_Main.SCM_Main" "/Game/Blueprints/SoundSettings/Sounds/SC_Music.SC_Music" (Variables|/Game/Blueprints/SoundSettings/BP_SaveSettings.BP_SaveSettings_C|GetMusicVolume (Variables|Default|GetSaveSettings)) 1.0 1.0 true)
      (Audio|SetSoundMixClassOverride "/Game/Blueprints/SoundSettings/Sounds/SCM_Main.SCM_Main" "/Game/Blueprints/SoundSettings/Sounds/SC_SFX.SC_SFX" (Variables|/Game/Blueprints/SoundSettings/BP_SaveSettings.BP_SaveSettings_C|GetSFXVolume (Variables|Default|GetSaveSettings)) 1.0 1.0 true)
      (Audio|PushSoundMixModifier "/Game/Blueprints/SoundSettings/Sounds/SCM_Main.SCM_Main"))
    (:Is%20Not%20Valid
      (Utilities|FlowControl|Delay 0.1)
      (goto _label))))

(event EventShutdown
  (SaveGame|SaveGametoSlot (Variables|Default|GetSaveSettings) "Settings"))

(fn GetGameInstanceSettings
  (return (Variables|Default|GetSaveSettings)))